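; BP_3D_Charts builds a 3D wave chart mesh procedurally in its construction script using Geometry Script on a dynamic mesh.
; GenerateWave produces a 2D profile from the sine toggle and length limit, which is extruded by Height into a solid.
; Triangles indexed up to the returned edge triangle count get a second material slot, giving the chart two materials.
; A cylinder mesh generation call is present but never runs.
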(fn `UserConstructionScript`
  (bind _returnvalue (`BaseDynamicMeshComponent.GetDynamicMesh` (`self.DynamicMesh`)))
  (bind (_out_vertices _edgetriangles _returnvalue_2) (`MeshOperationsBPLibrary.GenerateWave` (`self.Is Sin`) 30.0 50.0 (`self.Limit`)))
  (if _returnvalue_2
    (bind _returnvalue_3 (`GeometryScriptLibrary_MeshPrimitiveFunctions.AppendSimpleExtrudePolygon` _returnvalue (make `GeometryScriptPrimitiveOptions` "PerFace") (`self.Transform`) _out_vertices (`self.Height`) 0 true "Base" null))
    (for _index (range (+ _edgetriangles 1))
      (`GeometryScriptLibrary_MeshMaterialFunctions.SetTriangleMaterialID` _returnvalue_3 _index 1))
    (`PrimitiveComponent.SetMaterial` (`self.DynamicMesh`) 0 "/Engine/VREditor/BasicMeshes/MI_Cube_01.MI_Cube_01")
    (`PrimitiveComponent.SetMaterial` (`self.DynamicMesh`) 1 "/Engine/VREditor/BasicMeshes/MI_Cube_03.MI_Cube_03")))